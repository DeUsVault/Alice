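; BP_LaserGate is a laser gate actor that draws a stack of red Niagara beams, with no collision response or gameplay logic.
; On BeginPlay, a single Camera-channel line trace along the forward vector finds the first blocker within Distance.
; It spawns NumBeams attached NS_LaserGate systems spaced along local Y by BeamOffset.
; All share one local-space end point from the hit or maximum range, which is never updated afterward.
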(event EventBeginPlay
  (bind _returnvalue (Transformation|GetActorLocation))
  (bind _returnvalue_2 (Transformation|GetActorForwardVector))
  (bind _output_get (Variables|Default|SetTraceEnd (+ (* _returnvalue_2 (Variables|Default|GetDistance)) _returnvalue)))
  (bind _outhit (Collision|LineTraceByChannel (+ _returnvalue (* _returnvalue_2 "5.000000,5.000000,5.000000")) _output_get "TraceTypeQuery2" false 0 "None"))
  (Variables|Default|SetOut%20Hit%20Blocking%20Hit (.bblockinghit _outhit))
  (Variables|Default|SetOut%20Hit%20Location (Math|Transform|InverseTransformLocation (Transformation|GetActorTransform) (.location _outhit)))
  (for _index (range 0 (- (Variables|Default|GetNumBeams) 1))
    (Variables|Default|SetIndex _index)
    (bind _returnvalue_3 (Niagara|SpawnSystemAttached "/Game/Assets/FX/NS_LaserGate.NS_LaserGate" (Variables|Default|GetScene) "None" (* (Variables|Default|GetBeamOffset) (Math|Vector|MakeVector 0.0 (Variables|Default|GetIndex) 0.0)) "0, 0, 0" "KeepRelativeOffset" false))
    (Effects|Components|ParticleSystem|SetColorParameter _returnvalue_3 "LaserColour" "(R=1.000000,G=0.000000,B=0.000000,A=1.000000)")
    (Effects|Components|ParticleSystem|SetVectorParameter _returnvalue_3 "LaserEnd" (Math|Vector|SelectVector (Variables|Default|GetOut%20Hit%20Location) (Math|Transform|InverseTransformLocation (Transformation|GetActorTransform) (Variables|Default|GetTraceEnd)) (Variables|Default|GetOut%20Hit%20Blocking%20Hit)))))

(event Collision|EventActorBeginOverlap
  (params (OtherActor :type Actor%20Object%20Reference)))

(event EventTick
  (params (DeltaSeconds :type Float%20%28single-precision%29)))

(fn ConstructionScript)